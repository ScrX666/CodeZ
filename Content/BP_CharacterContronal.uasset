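; BP_CharacterContronal creates the player's Attack and HealthBar widgets and adds both to the viewport on BeginPlay.
; It reads Health from its AttributeComponent and prints it to the screen every Tick as debug output.
; The component's OnHealthChanged event also prints the new value in red, and nothing here passes health to the widgets.
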(event `self.ReceiveBeginPlay`
  (bind _returnvalue (`|CreateWidget` "/Game/UI/Attack.Attack_C"))
  (bind _returnvalue_2 (`|CreateWidget` "/Game/UI/HealthBar.HealthBar_C"))
  (`UserWidget.AddToViewport` _returnvalue 0)
  (`UserWidget.AddToViewport` _returnvalue_2 0))

(event `self.ReceiveTick`
  (params (DeltaSeconds :type "Float (single-precision)"))
  (`KismetSystemLibrary.PrintString` (`KismetStringLibrary.Conv_DoubleToString` (`SAttributeComponent.Health` (`self.AttributeComponent`))) true false (struct :`G` 0.66 :`B` 1.0 :`A` 1.0) 0.0))

(event `self.AttributeComponent.OnHealthChanged`
  (params (health :type "Float (single-precision)") (delta :type "Float (single-precision)") (instigetorActor :type "Actor Object Reference") (ownComp :type "SAttributeComponent Object Reference"))
  (`KismetSystemLibrary.PrintString` (`KismetStringLibrary.Conv_DoubleToString` health) true true (struct :`R` 1.0 :`B` 0.096454 :`A` 1.0)))

(fn `UserConstructionScript`)
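; BP_MagicProjectiled is a magic projectile actor that produces an impact effect when it hits something other than its instigator.
; On BeginPlay its sphere component ignores the instigator while moving.
; A valid hit draws a brief debug sphere, spawns the P_Priest_Stun particle effect at the projectile's location, then destroys the actor after a short delay.
; The graph applies no damage or stun logic.
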(event `self.ReceiveBeginPlay`
  (`PrimitiveComponent.IgnoreActorWhenMoving` (`self.SphereComponent`) (`self.Instigator`) true))

(event `self.SphereComponent.OnComponentHit`
  (params (HitComponent :type "PrimitiveComponent Object Reference") (OtherActor :type "Actor Object Reference") (OtherComp :type "PrimitiveComponent Object Reference") (NormalImpulse :type "Vector Structure") (Hit :type "HitResult Structure (by ref)"))
  (bind _returnvalue (`self.K2_GetActorLocation`))
  (if (!= (`self.Instigator`) OtherActor)
    (`KismetSystemLibrary.DrawDebugSphere` _returnvalue 10.0 12 (struct :`R` 1.0 :`B` 0.684247 :`A` 1.0) 0.5)
    (`GameplayStatics.SpawnEmitterAtLocation` "/Game/Art/RPGEffects/Particles/P_Priest_Stun.P_Priest_Stun" _returnvalue (`self.K2_GetActorRotation`))
    (`KismetSystemLibrary.Delay` 0.5)
    (`self.K2_DestroyActor`)))

(fn `UserConstructionScript`)